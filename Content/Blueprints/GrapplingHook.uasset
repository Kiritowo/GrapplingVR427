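; VR grappling hook projectile that pulls the VR character toward the point it hits.
; On sphere hit it stops its projectile movement, disables gravity on the character's capsule and opens a gate on Tick.
; Each tick the open gate applies a scaled force to the capsule, aimed from the motion controller to the hook.
; Destroying the hook re-enables the capsule's gravity.
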(event OnComponentHit(Sphere)
  (params (HitComponent :type Primitive%20Component%20Object%20Reference) (OtherActor :type Actor%20Object%20Reference) (OtherComp :type Primitive%20Component%20Object%20Reference) (NormalImpulse :type Vector :default "0, 0, 0") (Hit :type Hit%20Result%20Structure%20%28by%20ref%29))
  (Components|Movement|StopMovementImmediately (Variables|Default|GetProjectileMovement))
  (Physics|SetEnableGravity (Variables|/Script/Engine.Character|GetCapsuleComponent (Variables|Default|GetVRCharacter)) false)
  (Utilities|FlowControl|Gate true) ; enters at Open
)

(event EventTick
  (params (DeltaSeconds :type Float%20%28single-precision%29))
  (Utilities|FlowControl|Gate true
    (:Exit
      (Physics|AddForce (Variables|/Script/Engine.Character|GetCapsuleComponent (Variables|Default|GetVRCharacter)) (* (Math|Vector|GetForwardVector (Math|Rotator|FindLookatRotation (Transformation|GetWorldLocation (Variables|Default|GetMotionController)) (Transformation|GetActorLocation))) (Variables|Default|GetForce)) "None" false))))

(event EventDestroyed
  (Physics|SetEnableGravity (Variables|/Script/Engine.Character|GetCapsuleComponent (Variables|Default|GetVRCharacter)) true))

(fn ConstructionScript)