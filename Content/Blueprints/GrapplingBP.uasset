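; VR character Blueprint that fires a grappling hook from each hand's motion controller.
; Pressing a trigger spawns a scaled-down GrapplingHook actor at that controller's transform and passes it references to the character and controller.
; Releasing the trigger destroys that hand's hook, so left and right hooks work independently, with the grapple behavior left to the hook actor.
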(event Input|ActionEvents|InputActionTriggerLeft
  (params (Key :type Key%20Structure :default "None"))
  (bind _motioncontrollerleft (Variables|Default|GetMotionControllerLeft))
  (bind _returnvalue (Transformation|GetWorldTransform _motioncontrollerleft))
  (:Pressed
    (bind _returnvalue_2 (Game|SpawnActorfromClass "/Game/Blueprints/GrapplingHook.GrapplingHook_C" (Math|Transform|MakeTransform (.location _returnvalue) (.rotation _returnvalue) "0.100000,0.100000,0.100000") "AlwaysSpawn" 0 0))
    (bind _output_get (Variables|Default|SetLHook _returnvalue_2))
    (Variables|/Game/Blueprints/GrapplingHook.GrapplingHook_C|SetVRCharacter _output_get self)
    (Variables|/Game/Blueprints/GrapplingHook.GrapplingHook_C|SetMotionController _output_get (Variables|Default|GetMotionControllerLeft)))
  (:Released
    (Actor|DestroyActor (Variables|Default|GetLHook))))

(event Input|ActionEvents|InputActionTriggerRight
  (params (Key :type Key%20Structure :default "None"))
  (bind _motioncontrollerright (Variables|Default|GetMotionControllerRight))
  (bind _returnvalue (Transformation|GetWorldTransform _motioncontrollerright))
  (:Pressed
    (bind _returnvalue_2 (Game|SpawnActorfromClass "/Game/Blueprints/GrapplingHook.GrapplingHook_C" (Math|Transform|MakeTransform (.location _returnvalue) (.rotation _returnvalue) "0.100000,0.100000,0.100000") "AlwaysSpawn" 0 0))
    (bind _output_get (Variables|Default|SetRHook _returnvalue_2))
    (Variables|/Game/Blueprints/GrapplingHook.GrapplingHook_C|SetVRCharacter _output_get self)
    (Variables|/Game/Blueprints/GrapplingHook.GrapplingHook_C|SetMotionController _output_get (Variables|Default|GetMotionControllerRight)))
  (:Released
    (Actor|DestroyActor (Variables|Default|GetRHook))))

(fn ConstructionScript)